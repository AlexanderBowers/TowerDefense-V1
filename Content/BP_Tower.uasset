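; BP_Tower is a tower actor with early, test-stage logic for click-to-place movement.
; Clicking its static mesh toggles IsBeingPlaced; while set, Tick issues AIMoveTo through its AI controller every frame, using raw screen-space mouse coordinates as the goal's X and Y.
; A touch-begin handler traces Pawn objects under the cursor and prints debug text indicating whether it hit a BP_Tower.
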(event `self.ReceiveTick`
  (params (DeltaSeconds :type "Float (single-precision)"))
  (bind (_locationx _locationy) (`PlayerController.GetMousePosition` (`GameplayStatics.GetPlayerController` 0)))
  (if (`self.bIsBeingPlaced`)
    (`AITask_MoveTo.AIMoveTo` (`AIBlueprintHelperLibrary.GetAIController` self) (`KismetMathLibrary.MakeVector` _locationx _locationy) null)))

(event `self.ReceiveBeginPlay`
  (add `self.OnInputTouchBegin` (delegate `OnInputTouchBegin_Event`)))

(event `OnInputTouchBegin_Event` :!signature `self.OnInputTouchBegin`
  (params (FingerIndex :type "ETouchIndex Enum" :default "Touch1") (TouchedActor :type "Actor Object Reference"))
  (cast `/Game/BP_Tower` (`.HitActor` (`GameplayStatics.BreakHitResult` (`PlayerController.GetHitResultUnderCursorForObjects` (`GameplayStatics.GetPlayerController` 0) (`|MakeArray` "ObjectTypeQuery3" :!type "EObjectTypeQuery Enum") true)))
    (:`then`
      (`KismetSystemLibrary.PrintText` "Hello"))
    (:`CastFailed`
      (`KismetSystemLibrary.PrintText` "Nope!!!"))))

(event `self.StaticMesh.OnClicked`
  (params (TouchedComponent :type "PrimitiveComponent Object Reference") (ButtonPressed :type "Key Structure"))
  (set `self.bIsBeingPlaced` (not (`self.bIsBeingPlaced`))))

(fn `UserConstructionScript`)