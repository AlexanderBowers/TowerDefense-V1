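; BP_TowerHUD is a Blueprint that puts tower HUD arrow widgets on screen and turns the player's view target when clicked.
; BeginPlay creates two BPW_Arrow widgets, stored as Arrow and AddTower, and adds both to the player screen.
; OnClicked_Event rotates player 0's view target a quarter turn in yaw from the current viewpoint, keeping pitch and roll; no binding for this event appears in the graph.
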(event `self.ReceiveBeginPlay`
  (bind _returnvalue (`|CreateWidget` "/Game/BPW_Arrow.BPW_Arrow_C"))
  (bind _output_get (set `self.Arrow` _returnvalue))
  (`UserWidget.AddToPlayerScreen` _output_get 0)
  (bind _returnvalue_2 (`|CreateWidget` "/Game/BPW_Arrow.BPW_Arrow_C"))
  (bind _output_get_2 (set `self.Add Tower` _returnvalue_2))
  (`UserWidget.AddToPlayerScreen` _output_get_2 0))

(event `OnClicked_Event`
  (params (TouchedActor :type "Actor Object Reference") (ButtonPressed :type "Key Structure" :default "None"))
  (bind _returnvalue (`GameplayStatics.GetPlayerController` 0))
  (bind (_location _rotation) (`Controller.GetPlayerViewPoint` _returnvalue))
  (`self.K2_SetActorRotation` (`Controller.GetViewTarget` _returnvalue) (`KismetMathLibrary.MakeRotator` (.roll _rotation) (.pitch _rotation) (+ (.yaw _rotation) -90.0)) false))

(fn `UserConstructionScript`)